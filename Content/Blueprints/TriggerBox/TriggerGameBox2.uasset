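; Trigger box for a target-shooting minigame that binds its start event to the overlapping first-person character.
; On start, ShootingStyle either calls DontWantToThinkAboutIt for three-target random or runs a once-only "Only One Is Safe" spawn.
; That spawn puts a good target on a random TargetPoint and bad ones elsewhere, but rolls index and position separately.
; Tick's TargetPoint search goes unused, and the plane-rotation timeline update is unwired.
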(event `self.ReceiveBeginPlay`
  (`TimelineComponent.SetPlayRate` (`self.TheCircleMotion`) 0.5))

(event `self.ReceiveActorBeginOverlap`
  (params (OtherActor :type "Actor Object Reference"))
  (if (== (`GameplayStatics.GetObjectClass` OtherActor) "/Game/FirstPersonBP/Blueprints/FirstPersonCharacter.FirstPersonCharacter_C")
    (bind _asfirst_person_character (cast `/Game/FirstPersonBP/Blueprints/FirstPersonCharacter` OtherActor))
    (add `/Game/FirstPersonBP/Blueprints/FirstPersonCharacter.StartGame` _asfirst_person_character (delegate `startGame_CE`))))

(event `startGame_CE`
  (switch `/Game/Blueprints/TriggerBox/ShootingStyle` (`self.ShootingStyle`)
    (:`NewEnumerator0`
      (`self.DontWantToThinkAboutIt`))
    (:`NewEnumerator1`
      (`self.OnlyOneIsSafe`))))

(event `self.ReceiveTick`
  (params (DeltaSeconds :type "Float (single-precision)"))
  (bind _outactors (`GameplayStatics.GetAllActorsOfClass` "/Script/Engine.TargetPoint")))

(event `OnlyOneIsSafe`
  (`/Engine/EditorBlueprintResources/StandardMacros.DoOnce` false
    (:`Completed`
      (bind _outactors (`GameplayStatics.GetAllActorsOfClass` "/Script/Engine.TargetPoint"))
      (`|ExecutionSequence`
        (:`then_0`
          (bind _returnvalue (`KismetMathLibrary.RandomIntegerInRange` 0 (- (`KismetArrayLibrary.Array_Length` _outactors) 1)))
          (set `self.GoodTargetIndex` _returnvalue)
          (bind _returnvalue_2 (`|SpawnActorFromClass` "/Game/Blueprints/Targets/TargetTest.TargetTest_C" (`self.GetTransform` (`|GetArrayItem` _outactors _returnvalue)) "Undefined" "OverrideRootScale" null null))
          (`KismetArrayLibrary.Array_Add` (`self.SpawnActorArray`) _returnvalue_2))
        (:`then_1`
          (for (_array_element _array_index) _outactors
            (if (!= _array_index (`self.GoodTargetIndex`))
              (bind _returnvalue_3 (`|SpawnActorFromClass` "/Game/Blueprints/Targets/TargetBad.TargetBad_C" (`self.GetTransform` _array_element) "Undefined" "OverrideRootScale" null null))
              (`KismetArrayLibrary.Array_Add` (`self.SpawnBadActor`) _returnvalue_3))))))))

(event `3RandomTarget_CE`
  (bind _threetargets (`self.ThreeTargets`))
  (bind _outactors (`GameplayStatics.GetAllActorsOfClass` "/Script/Engine.TargetPoint"))
  (for _array_element _outactors
    (bind _returnvalue (`KismetStringLibrary.Conv_StringToName` (`KismetSystemLibrary.GetDisplayName` _array_element)))
    (if (or (== _returnvalue "TargetPoint") (== _returnvalue "TargetPoint2") (== _returnvalue "TargetPoint3"))
      (`KismetArrayLibrary.Array_Add` _threetargets _array_element)
      (if (== (`KismetArrayLibrary.Array_Length` _threetargets) 3)
        (`|SpawnActorFromClass` "/Game/Blueprints/Targets/TargetTest.TargetTest_C" (`self.GetTransform` (`|GetArrayItem` _threetargets (`KismetMathLibrary.RandomIntegerInRange` 0 2))) "Undefined" "OverrideRootScale" null null)))))

(fn `UserConstructionScript`)