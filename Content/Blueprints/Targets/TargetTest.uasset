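; TargetTest is a test target actor built around a WoodenBarrel1 component that explodes when overlapped and expires if left untouched.
; An overlap on the barrel prints the object name, spawns an attached explosion emitter and sound, then destroys the actor after a short delay.
; Independently, BeginPlay starts a timeout that plays a different explosion sound without particles and destroys the actor.
; Both sounds play at world origin.
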(event `self.WoodenBarrel1.OnComponentBeginOverlap`
  (params (OverlappedComponent :type "PrimitiveComponent Object Reference") (OtherActor :type "Actor Object Reference") (OtherComp :type "PrimitiveComponent Object Reference") (OtherBodyIndex :type Integer) (bFromSweep :type Boolean) (SweepResult :type "HitResult Structure (by ref)"))
  ;[1 1 1] If Hit
  (`KismetSystemLibrary.PrintString` (`KismetSystemLibrary.GetObjectName` null))
  (`GameplayStatics.SpawnEmitterAttached` "/Game/StarterContent/Particles/P_Explosion.P_Explosion")
  (`GameplayStatics.SpawnSoundAtLocation` "/Game/StarterContent/Audio/Explosion01.Explosion01")
  (`KismetSystemLibrary.Delay` 0.3)
  (`self.K2_DestroyActor`))

(event `self.ReceiveBeginPlay`
  ;[1 1 1] No hit
  (`KismetSystemLibrary.Delay` 5.0)
  (`GameplayStatics.PlaySoundAtLocation` "/Game/StarterContent/Audio/Explosion_Cue.Explosion_Cue")
  (`KismetSystemLibrary.Delay` 0.3)
  (`KismetSystemLibrary.PrintString` "Destroying")
  (`self.K2_DestroyActor`))

(fn `UserConstructionScript`)