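; Pop-up target spawner that cycles waves of targets across three spots: its own location and one either side along world X.
; Each wave randomly spawns either all TargetBad or one TargetTest with TargetBad elsewhere, though separate random rolls can make the good target overlap a bad one.
; Tick destroys the wave after a delay, then Reload spawns the next.
; The flip-up rotation timeline and older spawn chains are unconnected.
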(event `Load New`
  (bind _locations (`self.Locations`))
  (bind _returnvalue (`KismetMathLibrary.RandomIntegerInRange` 0 (- (`KismetArrayLibrary.Array_Length` _locations) 1)))
  (if (`KismetMathLibrary.RandomBool`) :!label _label
    (set `self.Bool1` true)
    (set `self.GoodTargetIndex` _returnvalue)
    (bind _returnvalue_2 (`|SpawnActorFromClass` "/Game/Blueprints/Targets/TargetTest.TargetTest_C" (`|GetArrayItem` _locations _returnvalue) "Undefined" "OverrideRootScale" null null))
    (set `self.NewVar_0` _returnvalue_2)
    (for (_array_element _array_index) _locations
      (if (!= _array_index (`self.GoodTargetIndex`))
        (bind _returnvalue_3 (`|SpawnActorFromClass` "/Game/Blueprints/Targets/TargetBad.TargetBad_C" _array_element "Undefined" "OverrideRootScale" null null))
        (`KismetArrayLibrary.Array_Add` (`self.NewVar_1`) _returnvalue_3)))
    (else
      (set `self.Bool1` true)
      (for _array_element_2 (`self.Locations`)
        (bind _returnvalue_4 (`|SpawnActorFromClass` "/Game/Blueprints/Targets/TargetBad.TargetBad_C" _array_element_2 "Undefined" "OverrideRootScale" null null))
        (`KismetArrayLibrary.Array_Add` (`self.NewVar_1`) _returnvalue_4)))))

(event `Reload`
  (`KismetSystemLibrary.Delay` 0.2)
  (goto _label))

(event `self.ReceiveTick`
  (params (DeltaSeconds :type "Float (single-precision)"))
  (if (`self.Bool1`)
    (`KismetSystemLibrary.Delay` 6.0)
    (`|ExecutionSequence`
      (:`then_0`
        (for _array_element (`self.NewVar_1`)
          (`self.K2_DestroyActor` _array_element)))
      (:`then_1`
        (`self.K2_DestroyActor` (`self.NewVar_0`)))
      (:`then_2`
        (`self.Reload`))
      (:`then_3`
        (set `self.Bool1` false)))))

(event `self.ReceiveBeginPlay`
  (bind _location (.location (`SceneComponent.K2_GetComponentToWorld` (`self.DefaultSceneRoot`))))
  (`|ExecutionSequence`
    (:`then_0`
      (set `self.Locations` (`|MakeArray` (`KismetMathLibrary.MakeTransform` _location) (`KismetMathLibrary.MakeTransform` (+ _location (300.0 0.0 0.0)) (struct) (1.0 1.0 1.0)) (`KismetMathLibrary.MakeTransform` (+ _location (-300.0 0.0 0.0))))))
    (:`then_1`
      (`self.Load New`))))

(fn `UserConstructionScript`
  (`self.K2_SetActorRotation` self (struct :`Pitch` -90.0 :`Yaw` 90.0) false))