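; Destructible cube Blueprint that breaks when hit by a first-person projectile.
; On a component hit from an actor tagged "Bullet", it enables physics simulation on the destructible component and applies radial damage at the impact point.
; Other hits increment an IsStacked counter, but its threshold check is left unconnected, so the count has no effect here.
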(event `self.Destructible.OnComponentHit`
  (params (HitComponent :type "PrimitiveComponent Object Reference") (OtherActor :type "Actor Object Reference") (OtherComp :type "PrimitiveComponent Object Reference") (NormalImpulse :type "Vector Structure") (Hit :type "HitResult Structure (by ref)"))
  ;[1 1 1] Destroy cube with FirstPersonProjectile
  (if (`self.ActorHasTag` OtherActor "Bullet")
    (`PrimitiveComponent.SetSimulatePhysics` (`self.Destructible`) true)
    (`GameplayStatics.ApplyRadialDamage` :`BaseDamage` 10.0 :`Origin` (`.ImpactPoint` (`GameplayStatics.BreakHitResult` Hit)) :`DamageRadius` 60.0 :`DamageTypeClass` "/Script/Engine.DamageType" :`bDoFullDamage` true)
    (else
      (set `self.IsStacked` (+ (`self.IsStacked`) 1.0)))))

(fn `UserConstructionScript`)